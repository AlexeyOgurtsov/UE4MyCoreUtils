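; BP_TestProjectile is a test projectile for the static gun in the projectile demo.
; On BeginPlay it calls InitProjectileMovement, which sets the ProjectileMovement velocity to the actor's forward vector times the component's initial speed.
; The function also prints and logs the forward vector for debugging, while overlap and tick events are unused.
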(event EventBeginPlay
  (|CallParentFunction)
  (Utilities|FlowControl|Sequence
    (:then_0
      (CallFunction|InitProjectileMovement))))

(event Collision|EventActorBeginOverlap
  (params (OtherActor :type Actor%20Object%20Reference)))

(event EventTick
  (params (DeltaSeconds :type Float%20%28single-precision%29)))

(fn ConstructionScript)

(fn InitProjectileMovement
  (bind _returnvalue (Transformation|GetActorRotation))
  (bind _returnvalue_2 (Math|Vector|GetForwardVector _returnvalue))
  (Variables|/Script/Engine.MovementComponent|SetVelocity (Variables|Default|GetProjectileMovement) (* _returnvalue_2 (Variables|/Script/Engine.ProjectileMovementComponent|GetInitialSpeed (Variables|Default|GetProjectileMovement))))
  (Utilities|FlowControl|Sequence
    (:then_0
      (Development|PrintString "InitPrjectileMovement"))
    (:then_1
      (Class|LogUtilLib|LogVector "GetActorRotation().GetForwardVector()" _returnvalue_2))))